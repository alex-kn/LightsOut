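; BP_EnemySpawner spawns BP_EnemyCharacterNew AI pawns inside its SpawnVolume box while the game mode still has enemies left to spawn.
; Each Tick it reads EnemiesToSpawn on BP_FirstPersonGameMode and, if above zero, decrements it and spawns one enemy at a random point in the volume.
; The game mode counter drives the spawning, so requested enemies appear at one per frame, with failure on collision disabled.
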(event `self.ReceiveTick`
  (params (DeltaSeconds :type "Float (single-precision)"))
  (bind _spawnvolume (`self.SpawnVolume`))
  ;[1 1 1] SpawnWhileEnemiesMissing
  (bind _asbp_first_person_game_mode (cast `/Game/LightsOut/Core/GameMode/BP_FirstPersonGameMode` (`GameplayStatics.GetGameMode`)))
  (bind _enemiestospawn (`/Game/LightsOut/Core/GameMode/BP_FirstPersonGameMode.EnemiesToSpawn` _asbp_first_person_game_mode))
  (if (> _enemiestospawn 0)
    (bind _result (`/Engine/EditorBlueprintResources/StandardMacros.DecrementInt` _enemiestospawn)
      (:`  `
        (set `/Game/LightsOut/Core/GameMode/BP_FirstPersonGameMode.EnemiesToSpawn` _result _asbp_first_person_game_mode)
        (`AIBlueprintHelperLibrary.SpawnAIFromClass` "/Game/LightsOut/Characters/Enemy/BP_EnemyCharacterNew.BP_EnemyCharacterNew_C" null (`KismetMathLibrary.RandomPointInBoundingBox` (`SceneComponent.K2_GetComponentLocation` _spawnvolume) (`BoxComponent.GetScaledBoxExtent` _spawnvolume)) (struct) true)))))

(fn `UserConstructionScript`)