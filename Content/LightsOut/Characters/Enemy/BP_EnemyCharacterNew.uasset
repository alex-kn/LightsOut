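; BP_EnemyCharacterNew is a zombie enemy that drains player health during Tick, gated by an attack distance check.
; Bullet-tagged overlaps on Head and Body deal different damage, with headshots hitting harder.
; Death updates the game mode's zombie count, plays an animation, awards the player money, disables collision and destroys the corpse after a delay.
; The construction script randomizes walk speed, and the Hit event only casts to the projectile.
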(event `/Game/LightsOut/Characters/iDamageable.AffectHealth`
  (params (Damage :type "Float (single-precision)"))
  (bind _moneyearned (`self.MoneyEarned`))
  ;[1 1 1] Get Damage
  (if (not (`self.isDead`))
    (`self.CalculateHealth` Damage)
    (if (`self.isDead`)
      (bind _asbp_first_person_game_mode (cast `/Game/LightsOut/Core/GameMode/BP_FirstPersonGameMode` (`GameplayStatics.GetGameMode`)))
      (`/Game/LightsOut/Core/GameMode/BP_FirstPersonGameMode.DecrementZombies` _asbp_first_person_game_mode)
      (`SkeletalMeshComponent.PlayAnimation` (`self.Mesh`) "/Game/ZombieGuy/Animations/Anim_Death_ZombieGuy.Anim_Death_ZombieGuy" false)
      ;[1 1 1] Give Player Cash
      (bind _asbase_character (cast `BaseCharacter` (`GameplayStatics.GetPlayerCharacter` 0)))
      (`self.CalculateMoney` _asbase_character _moneyearned)
      (bind _asbp_first_person_game_mode_2 (cast `/Game/LightsOut/Core/GameMode/BP_FirstPersonGameMode` (`GameplayStatics.GetGameMode`)))
      (`/Game/LightsOut/Core/GameMode/BP_FirstPersonGameMode.MoneyHasChanged` _asbp_first_person_game_mode_2 _moneyearned)
      ;[1 1 1] Make Corpse Disappear
      (`AudioComponent.Stop` (`self.Audio`))
      (`PrimitiveComponent.SetCollisionEnabled` (`self.Body`) "NoCollision")
      (`PrimitiveComponent.SetCollisionEnabled` (`self.CapsuleComponent`) "NoCollision")
      (`PrimitiveComponent.SetCollisionEnabled` (`self.Head`) "NoCollision")
      (`PrimitiveComponent.SetCollisionEnabled` (`self.Mesh`) "NoCollision")
      (`KismetSystemLibrary.Delay` 10.0)
      (`self.K2_DestroyActor`))))

(event `self.ReceiveTick`
  (params (DeltaSeconds :type "Float (single-precision)"))
  (bind _returnvalue (`GameplayStatics.GetPlayerCharacter` 0))
  (bind _returnvalue_2 (`self.GetDistanceTo` self _returnvalue))
  ;[1 1 1] Deal Damage
  (if (and (> _returnvalue_2 10.0) (< _returnvalue_2 150.0) (not (`self.isDead`)))
    (bind _asbp_first_person_character (cast `/Game/LightsOut/Core/Player/BP_FirstPersonCharacter` _returnvalue))
    (`/Game/LightsOut/Core/Player/BP_FirstPersonCharacter.AffectHealth` _asbp_first_person_character (* DeltaSeconds -10.0))))

(event `self.Head.OnComponentBeginOverlap`
  (params (OverlappedComponent :type "PrimitiveComponent Object Reference") (OtherActor :type "Actor Object Reference") (OtherComp :type "PrimitiveComponent Object Reference") (OtherBodyIndex :type Integer) (bFromSweep :type Boolean) (SweepResult :type "HitResult Structure (by ref)"))
  ;[1 1 1] Take Damage
  (if (`self.ActorHasTag` OtherActor "Bullet")
    (`self.AffectHealth` -100.0)
    (`self.K2_DestroyActor` OtherActor)))

(event `self.Body.OnComponentBeginOverlap`
  (params (OverlappedComponent :type "PrimitiveComponent Object Reference") (OtherActor :type "Actor Object Reference") (OtherComp :type "PrimitiveComponent Object Reference") (OtherBodyIndex :type Integer) (bFromSweep :type Boolean) (SweepResult :type "HitResult Structure (by ref)"))
  ;[1 1 1] Take Damage
  (if (`self.ActorHasTag` OtherActor "Bullet")
    (`self.AffectHealth` -20.0)
    (`self.K2_DestroyActor` OtherActor)))

(event `self.ReceiveHit`
  (params (MyComp :type "PrimitiveComponent Object Reference") (Other :type "Actor Object Reference") (OtherComp :type "PrimitiveComponent Object Reference") (bSelfMoved :type Boolean) (HitLocation :type "Vector Structure") (HitNormal :type "Vector Structure") (NormalImpulse :type "Vector Structure") (Hit :type "HitResult Structure (by ref)"))
  (cast `/Game/LightsOut/Core/Weapons/BP_Projectile` Other))

(fn `UserConstructionScript`
  (set `CharacterMovementComponent.MaxWalkSpeed` (`KismetMathLibrary.Conv_IntToDouble` (`KismetMathLibrary.RandomIntegerInRange` 200 300)) (`self.CharacterMovement`)))