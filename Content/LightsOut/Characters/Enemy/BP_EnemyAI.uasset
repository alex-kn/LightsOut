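; AI controller for enemy characters that makes them chase the player.
; A looping one-second timer started on BeginPlay calls TrackPlayer, which casts the controlled pawn to BP_EnemyCharacterNew and checks IsDead.
; Living enemies get an AI MoveTo targeting player character 0.
; Dead ones trigger a move to their own location, though that node's Pawn input is unset.
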(event `self.ReceiveBeginPlay`
  (`KismetSystemLibrary.K2_SetTimer` null "TrackPlayer" 1.0 true))

(event `TrackPlayer`
  (bind _asbp_enemy_character_new (cast `/Game/LightsOut/Characters/Enemy/BP_EnemyCharacterNew` (`self.K2_GetPawn`)))
  (if (`BaseCharacter.isDead` _asbp_enemy_character_new)
    (`|AIMoveTo` null (`self.K2_GetActorLocation` (`self.K2_GetPawn`)))
    (else
      (`|AIMoveTo` (`self.K2_GetPawn`) (0.0 0.0 0.0) (`GameplayStatics.GetPlayerCharacter` 0)))))

(fn `UserConstructionScript`)