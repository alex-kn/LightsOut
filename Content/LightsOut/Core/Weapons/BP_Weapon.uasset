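; BP_Weapon is the player's magazine-fed gun, tracking rounds and spare magazines and playing fire and reload animations and sounds.
; PullTrigger spawns BP_Projectile unless the character holds an object or a reload is running, and dry-fires when empty.
; Releasing R spends a magazine, refills rounds immediately and blocks firing until a timer ends.
; Projectile rotation gets random spray from player movement and shots under half a second apart, scaled by that interval.
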(event `AddMagazine`
  ;[1 1 1] Add Magazine
  (set `self.Magazines` (+ (`self.Magazines`) 1)))

(event `self.ReceiveBeginPlay`
  ;[1 1 1] Begin Play & Setup
  (`self.EnableInput` (`GameplayStatics.GetPlayerController` 0))
  (`self.ConfigureWeapon`))

(event `ConfigureWeapon`
  ;[1 1 1] Setup Weapon
  (bind _output_get (set `self.InitialMagazines` 5))
  (set `self.Magazines` _output_get)
  (bind _output_get_2 (set `self.RoundsPerMagazine` 30))
  (set `self.RoundsLeftInMagazine` _output_get_2)
  (set `self.RoundsPerSecond` 7.0)
  (set `self.ReloadingTime` 1.5))

(event `PullTrigger`
  ;[1 1 1] Shooting
  (`self.Fire`))

(event `Fire`
  ;[1 1 1] Shooting
  (bind _asbp_first_person_character (cast `/Game/LightsOut/Core/Player/BP_FirstPersonCharacter` (`GameplayStatics.GetPlayerCharacter` 0)))
  (if (or (`/Game/LightsOut/Core/Player/BP_FirstPersonCharacter.bIsHoldingObject` _asbp_first_person_character) (`self.isReloading`))
    _
    (elif (> (`self.RoundsLeftInMagazine`) 0)
      (set `self.RoundsLeftInMagazine` (- (`self.RoundsLeftInMagazine`) 1))
      (`SkeletalMeshComponent.PlayAnimation` (`self.SkeletalMesh`) "/Game/IBWP3DG18/Weapons/G18/Animations/ANIM_G18_Fire_Montage.ANIM_G18_Fire_Montage" false)
      (bind _newparam (`self.getWorldTransformWithSprayAndRecoil`))
      (`|SpawnActorFromClass` "/Game/LightsOut/Core/Weapons/BP_Projectile.BP_Projectile_C" _newparam "AlwaysSpawn" "OverrideRootScale")
      (`GameplayStatics.PlaySoundAtLocation` "/Game/LightsOut/Weapons/StandardWeapon/9_mm_gunshot.9_mm_gunshot" (`self.K2_GetActorLocation`))
      (set `self.TimeAtLastShot` (`GameplayStatics.GetTimeSeconds`))
      (else
        (`GameplayStatics.PlaySoundAtLocation` "/Game/LightsOut/Weapons/StandardWeapon/Dry_Fire.Dry_Fire" (`self.K2_GetActorLocation`))))))

(event `Key|R`
  (params (Key :type "Key Structure" :default "AnyKey"))
  ;[1 1 1] Reload
  (:`Released`
    (if (> (`self.Magazines`) 0)
      (set `self.isReloading` true)
      (set `self.Magazines` (- (`self.Magazines`) 1))
      (set `self.RoundsLeftInMagazine` (`self.RoundsPerMagazine`))
      (`GameplayStatics.PlaySoundAtLocation` "/Game/LightsOut/Weapons/StandardWeapon/A_Reload.A_Reload" (`self.K2_GetActorLocation`))
      (`SkeletalMeshComponent.PlayAnimation` (`self.SkeletalMesh`) "/Game/IBWP3DG18/Weapons/G18/Animations/ANIM_G18_Reload_Montage.ANIM_G18_Reload_Montage" false)
      (`KismetSystemLibrary.K2_SetTimer` null "resetReloading" (`self.ReloadingTime`)))))

(fn `getWorldTransformWithSprayAndRecoil`
  (returns (NewParam :type "Transform Structure"))
  (bind _returnvalue (- (`GameplayStatics.GetTimeSeconds`) (`self.TimeAtLastShot`)))
  (bind _returnvalue_2 (* _returnvalue 10.0))
  (bind _returnvalue_3 (`KismetMathLibrary.RandomFloatInRange` (* _returnvalue_2 -1.0) _returnvalue_2))
  ;[1 1 1] Check Fire Rate; More than 2 per second create Spray
  (if (>= _returnvalue 0.5)
    (set `self.TempRotationFireRate` (`KismetMathLibrary.MakeRotator` 0.0))
    (else
      (set `self.TempRotationFireRate` (`KismetMathLibrary.MakeRotator` _returnvalue_3 _returnvalue_3 _returnvalue_3))))
  ;[1 1 1] Check Movement; If Moving add Spray
  (bind _asbp_first_person_character (cast `/Game/LightsOut/Core/Player/BP_FirstPersonCharacter` (`GameplayStatics.GetPlayerCharacter` 0)))
  (bind _newparam (`/Game/LightsOut/Core/Player/BP_FirstPersonCharacter.IsMoving` _asbp_first_person_character))
  (if _newparam
    (set `self.TempRotationMovement` (`KismetMathLibrary.MakeRotator` (`KismetMathLibrary.RandomFloatInRange` -2.0 2.0) (`KismetMathLibrary.RandomFloatInRange` -2.0 2.0) (`KismetMathLibrary.RandomFloatInRange` -2.0 2.0))))
  (return (`KismetMathLibrary.MakeTransform` (`SceneComponent.K2_GetComponentLocation` (`self.ProjectileSpawnPoint`)) (`KismetMathLibrary.MakeRotator` (+ (+ (.roll (`SceneComponent.K2_GetComponentRotation` (`self.ProjectileSpawnPoint`))) (.roll (`self.TempRotationFireRate`))) (.roll (`self.TempRotationMovement`))) (+ (+ (.pitch (`SceneComponent.K2_GetComponentRotation` (`self.ProjectileSpawnPoint`))) (.pitch (`self.TempRotationFireRate`))) (.pitch (`self.TempRotationMovement`))) (+ (+ (.yaw (`SceneComponent.K2_GetComponentRotation` (`self.ProjectileSpawnPoint`))) (.yaw (`self.TempRotationFireRate`))) (.yaw (`self.TempRotationMovement`)))) (1.0 1.0 1.0))))

(fn `NewFunction_0`)

(fn `resetReloading`
  (set `self.isReloading` false))

(fn `UserConstructionScript`)