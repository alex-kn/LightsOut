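; Base shop actor that shows a buy prompt when the player overlaps it and handles Buy input.
; BeginPlay enables input and caches the first-person character and game mode, which displays the prompt.
; Pressing Buy inside ActivationRadius calls StartBuy, while releasing calls StopBuy without a range check.
; Both functions are empty, apparently hooks for child shops to implement the purchase.
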(event `self.ReceiveActorBeginOverlap`
  (params (OtherActor :type "Actor Object Reference"))
  (if (== OtherActor (`self.PlayerCharacter`))
    (`/Game/LightsOut/Core/GameMode/BP_FirstPersonGameMode.ShowTextMessage` (`self.FirstPersonGameMode`) (`self.BuyInfoMessage`))))

(event `self.ReceiveBeginPlay`
  (`self.EnableInput` (`GameplayStatics.GetPlayerController` 0))
  (bind _asbp_first_person_character (cast `/Game/LightsOut/Core/Player/BP_FirstPersonCharacter` (`GameplayStatics.GetPlayerCharacter` 0)))
  (set `self.PlayerCharacter` _asbp_first_person_character)
  (bind _asbp_first_person_game_mode (cast `/Game/LightsOut/Core/GameMode/BP_FirstPersonGameMode` (`GameplayStatics.GetGameMode`)))
  (set `self.FirstPersonGameMode` _asbp_first_person_game_mode))

(event `InputAction|Buy` :consume false
  (params (Key :type "Key Structure" :default "AnyKey"))
  (:`Pressed`
    (bind _playerisinshoparea (`self.isPlayerInShopArea`))
    (if _playerisinshoparea
      (`self.startBuy`)))
  (:`Released`
    (`self.stopBuy`)))

(fn `isPlayerInShopArea`
  (returns (playerIsInShopArea :type Boolean))
  (return (`PrimitiveComponent.IsOverlappingActor` (`self.ActivationRadius`) (`self.PlayerCharacter`))))

(fn `startBuy`)

(fn `stopBuy`)

(fn `UserConstructionScript`)