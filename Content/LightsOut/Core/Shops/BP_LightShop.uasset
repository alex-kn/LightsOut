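; BP_LightShop is a shop that sells lamps to the player, overriding a parent's construction script to set its buy prompt.
; StartBuy asks the player character to apply the negative Price through CalculateMoney.
; On success it notifies the game mode of the money change and spawns a BP_Lamp in front of the player, adjusting for collisions.
; On failure it has the game mode show a not-enough-money message.
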(event `self.startBuy`
  (bind _playercharacter (`self.PlayerCharacter`))
  (bind _returnvalue (* -1 (`self.Price`)))
  (bind _returnvalue_2 (`BaseCharacter.CalculateMoney` (`self.PlayerCharacter`) _returnvalue))
  (if _returnvalue_2
    (`/Game/LightsOut/Core/GameMode/BP_FirstPersonGameMode.MoneyHasChanged` (`self.FirstPersonGameMode`) _returnvalue)
    (`|SpawnActorFromClass` "/Game/LightsOut/Core/Pickupables/BP_Lamp.BP_Lamp_C" (`KismetMathLibrary.Conv_VectorToTransform` (+ (`self.K2_GetActorLocation` _playercharacter) (* (`self.GetActorForwardVector` _playercharacter) (`self.SpawnDistance`)))) "AdjustIfPossibleButAlwaysSpawn" "OverrideRootScale")
    (else
      (`/Game/LightsOut/Core/GameMode/BP_FirstPersonGameMode.ShowTextMessage` (`self.FirstPersonGameMode`) (`self.NotEnougMoneyMessage`)))))

(fn `UserConstructionScript`
  (`parent.UserConstructionScript`)
  (set `self.BuyInfoMessage` "Press >B< for some LIGHTS! "))