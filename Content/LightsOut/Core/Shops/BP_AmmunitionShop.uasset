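; BP_AmmunitionShop is a shop where the player buys extra ammunition for the weapon currently held.
; On StartBuy it asks the player character to validate the price, then notifies the game mode of the money change and adds a magazine to the current weapon.
; If funds are short, the game mode shows a not-enough-money message.
; The construction script runs its parent's and sets the buy prompt text.
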(event `self.startBuy`
  (bind _returnvalue (* -1 (`self.Price`)))
  (bind _returnvalue_2 (`BaseCharacter.CalculateMoney` (`self.PlayerCharacter`) _returnvalue))
  (if _returnvalue_2
    (`/Game/LightsOut/Core/GameMode/BP_FirstPersonGameMode.MoneyHasChanged` (`self.FirstPersonGameMode`) _returnvalue)
    (bind _weapon (`/Game/LightsOut/Core/Player/BP_FirstPersonCharacter.getCurrentWeapon` (`self.PlayerCharacter`)))
    (`/Game/LightsOut/Core/Weapons/BP_Weapon.AddMagazine` _weapon)
    (else
      (`/Game/LightsOut/Core/GameMode/BP_FirstPersonGameMode.ShowTextMessage` (`self.FirstPersonGameMode`) (`self.NotEnoughMoneyMessage`)))))

(fn `UserConstructionScript`
  (`parent.UserConstructionScript`)
  (set `self.BuyInfoMessage` "Press >B< to buy MOAR AMMO!  "))