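; BP_HealthShop is a shop that sells the player healing over time for money, with a "Press >B< to heal!" prompt.
; StartBuy runs a looping timer that each interval charges the player, adds health and notifies the game mode of the money change.
; StopBuy clears the timer, which also happens automatically with an on-screen message when health is full or money runs out.
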(event `self.startBuy`
  (bind _returnvalue (`KismetSystemLibrary.K2_SetTimerDelegate` (delegate `Buy Health`) (`self.IntervalTime`) true))
  (set `self.TimerHandle` _returnvalue))

(event `Buy Health`
  (if (not (`BaseCharacter.hasFullHealth` (`self.PlayerCharacter`)))
    (bind _returnvalue (`BaseCharacter.CalculateMoney` (`self.PlayerCharacter`) (* -1 (`self.PricePerInterval`))))
    (if _returnvalue
      (`BaseCharacter.CalculateHealth` (`self.PlayerCharacter`) (`self.HealAmountPerInterval`))
      (`/Game/LightsOut/Core/GameMode/BP_FirstPersonGameMode.MoneyHasChanged` (`self.FirstPersonGameMode`) (* -1 (`self.PricePerInterval`)))
      (else
        (`self.stopBuy`)
        (`/Game/LightsOut/Core/GameMode/BP_FirstPersonGameMode.ShowTextMessage` (`self.FirstPersonGameMode`) (`self.NotEnoughMoneyMessage`))))
    (else
      (`self.stopBuy`)
      (`/Game/LightsOut/Core/GameMode/BP_FirstPersonGameMode.ShowTextMessage` (`self.FirstPersonGameMode`) (`self.FullHealthMessage`)))))

(event `self.stopBuy`
  (`KismetSystemLibrary.K2_ClearAndInvalidateTimerHandle` (`self.TimerHandle`)))

(fn `UserConstructionScript`
  (`parent.UserConstructionScript`)
  (set `self.BuyInfoMessage` "Press >B< to heal!"))